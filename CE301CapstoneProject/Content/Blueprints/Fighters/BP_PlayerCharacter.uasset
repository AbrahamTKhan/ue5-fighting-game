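; Player fighter character Blueprint that handles per-player HUD, lock-on widget ownership and a material opacity effect.
; On possession it creates and shows a HUD on that player's screen, with an event to remove it.
; BeginPlay uses a throwaway widget to obtain the second local player and assign it as LockOnWidgetP2's owner.
; Dynamic material instances are cached from the mesh, and ShowTankFX drives their Opacity through a timeline.
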(event EventRemoveHUD
  (Widget|RemovefromParent (Variables|Default|GetPlayerHUD)))

(event Collision|EventActorBeginOverlap
  (params (OtherActor :type Actor%20Object%20Reference)))

(event EventTick
  (params (DeltaSeconds :type Float%20%28single-precision%29)))

(event EventPossessed
  (params (NewController :type Controller%20Object%20Reference))
  (Utilities|IsValid (Pawn|GetControlledPawn NewController)
    (:Is%20Valid
      (bind _asplayer_controller (Utilities|Casting|CastToPlayerController (Pawn|GetController)))
      (bind _returnvalue (UserInterface|CreateWidget "/Game/Blueprints/UI/Player/BP_HUD.BP_HUD_C" _asplayer_controller))
      (bind _output_get (Variables|Default|SetPlayerHUD _returnvalue))
      (UserInterface|Viewport|AddtoPlayerScreen _output_get))))

(event EventBeginPlay
  (bind _returnvalue (Class|GameplayStatics|GetPlayerControllerfromID 1))
  (Utilities|IsValid _returnvalue
    (:Is%20Valid
      (bind _returnvalue_2 (UserInterface|CreateWidget "/Game/Blueprints/UI/MainMenu/BackgroundWidget.BackgroundWidget_C" _returnvalue))
      (Widget|RemovefromParent _returnvalue_2)
      (Class|WidgetComponent|SetOwnerPlayer (Variables|Default|GetLockOnWidgetP2) (Class|Widget|GetOwningLocalPlayer _returnvalue_2)))))

(event EventShowTankFX
  (bind _newtrack_0 (Timeline|Mat%20Opacity%20Timeline PlayFromStart)
    (:Update
      (for _array_element (Variables|Default|GetMatVar)
        (Rendering|Material|SetScalarParameterValue _array_element "Opacity" _newtrack_0 :!class /Script/Engine.MaterialInstanceDynamic)))))

(event EventCreateDynamicMaterialInstances
  (for (_ _array_index) (Rendering|Material|GetMaterials (Variables|Character|GetMesh))
    (bind _returnvalue (Rendering|Material|CreateDynamicMaterialInstance (Variables|Character|GetMesh) _array_index 0 "None" :!class /Script/Engine.PrimitiveComponent))
    (Utilities|Array|Add (Variables|Default|GetMatVar) _returnvalue)))

(fn ConstructionScript)