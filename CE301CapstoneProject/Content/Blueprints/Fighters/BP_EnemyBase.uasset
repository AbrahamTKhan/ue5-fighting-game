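; Base enemy fighter that gives each local player their own health and stamina display in one- or two-player games.
; BeginPlay spawns UI actors owned by each player character and assigns the P2 lock-on widget's owner through a throwaway widget.
; UpdateHUD pushes health, Tick pushes stamina, and Unpossessed destroys the UI.
; ShowTankFX fades cached dynamic materials via timeline; older widget-component HUD logic remains disconnected.
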(event EventUnpossessed
  (params (OldController :type Controller%20Object%20Reference))
  (Actor|DestroyActor (Variables|Default|GetPlayer%20HUD))
  (if (Variables|Default|GetHas%20Local%20Player)
    (Actor|DestroyActor (Variables|Default|GetLocal%20Player%20HUD))))

(event EventUpdateHUD
  (Default|UpdateHealth (Variables|Default|GetPlayer%20HUD) (Class|FighterBase|GetHealth))
  (if (Variables|Default|GetHas%20Local%20Player)
    (Default|UpdateHealth (Variables|Default|GetLocal%20Player%20HUD) (Class|FighterBase|GetHealth))))

(event EventTick
  (params (DeltaSeconds :type Float%20%28single-precision%29))
  (if (Variables|Default|GetPlayer%201%20Confirmed)
    (Default|UpdateStamina (Variables|Default|GetPlayer%20HUD) (Class|FighterBase|GetStamina))
    (if (Variables|Default|GetHas%20Local%20Player)
      (Default|UpdateStamina (Variables|Default|GetLocal%20Player%20HUD) (Class|FighterBase|GetStamina)))))

(event EventBeginPlay
  (bind _returnvalue (Class|GameplayStatics|GetPlayerControllerfromID 1))
  (for (_ _array_index) (Rendering|Material|GetMaterials (Variables|Character|GetMesh))
    (bind _returnvalue_2 (Rendering|Material|CreateDynamicMaterialInstance (Variables|Character|GetMesh) _array_index 0 "None" :!class /Script/Engine.PrimitiveComponent))
    (Utilities|Array|Add (Variables|Default|GetMatVar) _returnvalue_2))
  (Utilities|FlowControl|Delay 0.1)
  (CallFunction|CreatePlayer1HUD)
  (Utilities|IsValid (Class|GameplayStatics|GetPlayerControllerfromID 1)
    (:Is%20Valid
      (Variables|Default|SetHas%20Local%20Player true)
      (CallFunction|CreatePlayer2HUD)
      (Utilities|IsValid _returnvalue
        (:Is%20Valid
          (bind _returnvalue_3 (UserInterface|CreateWidget "/Game/Blueprints/UI/MainMenu/BackgroundWidget.BackgroundWidget_C" _returnvalue))
          (Widget|RemovefromParent _returnvalue_3)
          (Class|WidgetComponent|SetOwnerPlayer (Variables|Default|GetLockOnWidgetP2) (Class|Widget|GetOwningLocalPlayer _returnvalue_3)))))
    (:Is%20Not%20Valid
      (Variables|Default|SetHas%20Local%20Player false))))

(event EventShowTankFX
  (bind _newtrack_0 (Timeline|Timeline_0 Play)
    (:Update
      (for _array_element (Variables|Default|GetMatVar)
        (Rendering|Material|SetScalarParameterValue _array_element "Opacity" _newtrack_0 :!class /Script/Engine.MaterialInstanceDynamic)))))

(fn ConstructionScript)

(fn RotateHUD1
  (Utilities|IsValid (Game|GetPlayerCameraManager 0)))

(fn RotateHUD2
  (bind _returnvalue (Game|GetPlayerCameraManager 1))
  (Utilities|IsValid _returnvalue
    (:Is%20Valid
      (Transformation|SetWorldRotation (Variables|Default|GetLocalHUD) (Math|Rotator|FindLookatRotation (Transformation|GetWorldLocation (Variables|Default|GetLocalHUD)) (Camera|GetCameraLocation _returnvalue)) false false))))

(fn CreatePlayer1HUD
  (bind _asbp_player_character (Utilities|Casting|CastToBP_PlayerCharacter (Game|GetPlayerCharacter 0)))
  (Utilities|IsValid (Class|GameplayStatics|GetPlayerControllerfromID)
    (:Is%20Valid
      (Variables|Default|SetPlayer%201%20Confirmed true)
      (bind _returnvalue (Game|SpawnActorfromClass "/Game/Blueprints/UI/EnemyUI.EnemyUI_C" (Transformation|GetActorTransform) "Undefined" _asbp_player_character 0))
      (bind _output_get (Variables|Default|SetPlayer%20HUD _returnvalue))
      (Default|SetEnemy _output_get self)
      (Default|SetStartingValues _output_get (Variables|Default|GetmaxHealth) (Variables|Default|GetmaxStamina))
      (Default|UpdateHealth (Variables|Default|GetPlayer%20HUD) (Class|FighterBase|GetHealth)))
    (:Is%20Not%20Valid
      (Variables|Default|SetPlayer%201%20Confirmed false))))

(fn CreatePlayer2HUD
  (bind _asbp_player_character (Utilities|Casting|CastToBP_PlayerCharacter (Game|GetPlayerCharacter 1)))
  (bind _returnvalue (Game|SpawnActorfromClass "/Game/Blueprints/UI/EnemyUI_Local.EnemyUI_Local_C" (Transformation|GetActorTransform) "Undefined" _asbp_player_character 0))
  (bind _output_get (Variables|Default|SetLocal%20Player%20HUD _returnvalue))
  (Default|SetEnemy _output_get self)
  (Default|SetStartingValues (Variables|Default|GetLocal%20Player%20HUD) (Variables|Default|GetmaxHealth) (Variables|Default|GetmaxStamina))
  (Utilities|Casting|CastToBP_PlayerFighterController (Class|GameplayStatics|GetPlayerControllerfromID))
  (Default|UpdateHealth (Variables|Default|GetLocal%20Player%20HUD) (Class|FighterBase|GetHealth)))