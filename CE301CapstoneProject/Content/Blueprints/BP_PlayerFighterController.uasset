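; Player controller for the fighter that runs the multi-level combat tutorial, from dialogue prompts to level progression.
; Tutorial dialogue disables character input and advances on ProgressDialogue; its box type then either restores input or fades to another level.
; Restoring input outside tutorial-0 shows a level-specific action counter and, in some levels, points enemies at the player.
; Update events count moves per level and, at thresholds, load the next level or show closing dialogue.
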(event Custom|Event%20Start%20Tutorial%20HUD
  (params (Text :type Array%20of%20Strings) (Type :type Integer) (Input%20Title :type String) (Input%20Text :type String))
  (Variables|Default|SetText%20Array Text)
  (Variables|Default|SetBox%20Type Type)
  (Variables|Default|SetInput%20Title Input%20Title)
  (Variables|Default|SetInput%20Text Input%20Text)
  (Variables|Default|SetMaxIndex (Utilities|Array|Length (Variables|Default|GetText%20Array)))
  (bind _returnvalue (UserInterface|CreateWidget "/Game/Blueprints/UI/Tutorial/TutorialPrompts.TutorialPrompts_C"))
  (bind _output_get (Variables|Default|SetTutorial%20Prompt _returnvalue))
  (UserInterface|Viewport|AddtoViewport _output_get 0)
  (Variables|Default|SetDialogueIndex 0)
  (Input|DisableInput (Game|GetPlayerCharacter 0) (Game|GetPlayerController 0))
  (if (> (Variables|Default|GetMaxIndex) 0)
    (Default|ChangeText (Variables|Default|GetTutorial%20Prompt) (Utilities|Array|Get(acopy) (Variables|Default|GetText%20Array)))
    (Default|ChangeInputText (Variables|Default|GetTutorial%20Prompt) (Variables|Default|GetInput%20Title) (Variables|Default|GetInput%20Text))))

(event EventUpdatePerfectBlocks
  (bind _returnvalue (Game|GetCurrentLevelName true))
  (if (Utilities|Enum|Equal(Enum) _returnvalue "tutorial-7")
    (bind _output_get (Variables|Default|SetPerfect%20Blocks (+ 1 (Variables|Default|GetPerfect%20Blocks))))
    (Default|ChangeCount1 (Variables|Default|GetAction%20Widget) (Utilities|String|ToString(Integer) _output_get))
    (if (>= _output_get 3)
      (CallFunction|CreateFade)
      (Utilities|FlowControl|Delay 1.0)
      (Game|OpenLevel(byName) "tutorial-8"))))

(event EventUpdateBlockBreakers
  (bind _returnvalue (Game|GetCurrentLevelName true))
  (if (Utilities|Enum|Equal(Enum) _returnvalue "tutorial-8")
    (bind _output_get (Variables|Default|SetBlock%20Breakers (+ 1 (Variables|Default|GetBlock%20Breakers))))
    (Default|ChangeCount1 (Variables|Default|GetAction%20Widget) (Utilities|String|ToString(Integer) _output_get))
    (if (>= _output_get 3)
      (CallFunction|CreateFade)
      (Utilities|FlowControl|Delay 1.0)
      (Game|OpenLevel(byName) "tutorial-9"))))

(event EventUpdateHeavyAttacks
  (bind _returnvalue (Game|GetCurrentLevelName true))
  (if (Utilities|Enum|Equal(Enum) _returnvalue "tutorial-1")
    (bind _output_get (Variables|Default|SetHeavy%20Attacks (+ 1 (Variables|Default|GetHeavy%20Attacks))))
    (Default|ChangeCount2 (Variables|Default|GetAction%20Widget) (Utilities|String|ToString(Integer) _output_get))
    (if (Math|Boolean|ANDBoolean (>= (stale EventUpdateLightAttacks _output_get) 2) (>= _output_get 2) (>= (stale EventUpdateSpecialAttacks _output_get) 1))
      (bind _newparam1 (CallFunction|CreateDialogues))
      (CallFunction|EventStartTutorialHUD _newparam1 2))))

(event EventUpdateSpecialAttacks
  (bind _returnvalue (Game|GetCurrentLevelName true))
  (if (Utilities|Enum|Equal(Enum) _returnvalue "tutorial-1")
    (bind _output_get (Variables|Default|SetSpecial%20Attacks (+ 1 (Variables|Default|GetSpecial%20Attacks))))
    (Default|ChangeCount3 (Variables|Default|GetAction%20Widget) (Utilities|String|ToString(Integer) _output_get))
    (if (Math|Boolean|ANDBoolean (>= (stale EventUpdateLightAttacks _output_get) 2) (>= (stale EventUpdateHeavyAttacks _output_get) 2) (>= _output_get 1))
      (bind _newparam1 (CallFunction|CreateDialogues))
      (CallFunction|EventStartTutorialHUD _newparam1 2))))

(event EventUpdateKickboxingAttacks
  (bind _returnvalue (Game|GetCurrentLevelName true))
  (if (Utilities|Enum|Equal(Enum) _returnvalue "tutorial-2")
    (bind _output_get (Variables|Default|SetKickboxing%20Attacks (+ 1 (Variables|Default|GetKickboxing%20Attacks))))
    (Default|ChangeCount1 (Variables|Default|GetAction%20Widget) (Utilities|String|ToString(Integer) _output_get))
    (if (and (>= _output_get 2) (>= (stale EventUpdateWeaponAttacks _output_get) 2))
      (CallFunction|CreateFade)
      (Utilities|FlowControl|Delay 1.0)
      (Game|OpenLevel(byName) "tutorial-3"))))

(event EventUpdateWeaponAttacks
  (bind _returnvalue (Game|GetCurrentLevelName true))
  (if (Utilities|Enum|Equal(Enum) _returnvalue "tutorial-2")
    (bind _output_get (Variables|Default|SetWeapon%20Attacks (+ 1 (Variables|Default|GetWeapon%20Attacks))))
    (Default|ChangeCount2 (Variables|Default|GetAction%20Widget) (Utilities|String|ToString(Integer) _output_get))
    (if (and (>= (stale EventUpdateKickboxingAttacks _output_get) 2) (>= _output_get 2))
      (CallFunction|CreateFade)
      (Utilities|FlowControl|Delay 1.0)
      (Game|OpenLevel(byName) "tutorial-3"))))

(event EventUpdateMagicAttacks
  (bind _returnvalue (Game|GetCurrentLevelName true))
  (if (Utilities|Enum|Equal(Enum) _returnvalue "tutorial-3")
    (bind _output_get (Variables|Default|SetMagic%20Attacks (+ 1 (Variables|Default|GetMagic%20Attacks))))
    (Default|ChangeCount1 (Variables|Default|GetAction%20Widget) (Utilities|String|ToString(Integer) _output_get))
    (if (>= _output_get 6)
      (CallFunction|CreateFade)
      (Utilities|FlowControl|Delay 1.0)
      (Game|OpenLevel(byName) "tutorial-4"))))

(event EventUpdateDodges
  (bind _returnvalue (Game|GetCurrentLevelName true))
  (if (Utilities|Enum|Equal(Enum) _returnvalue "tutorial-4")
    (bind _output_get (Variables|Default|SetDodges (+ 1 (Variables|Default|GetDodges))))
    (Default|ChangeCount1 (Variables|Default|GetAction%20Widget) (Utilities|String|ToString(Integer) _output_get))
    (if (>= _output_get 2)
      (CallFunction|CreateFade)
      (Utilities|FlowControl|Delay 1.0)
      (Game|OpenLevel(byName) "tutorial-5"))))

(event EventUpdateBlocks
  (bind _returnvalue (Game|GetCurrentLevelName true))
  (if (Utilities|Enum|Equal(Enum) _returnvalue "tutorial-5")
    (bind _output_get (Variables|Default|SetBlocks (+ 1 (Variables|Default|GetBlocks))))
    (Default|ChangeCount1 (Variables|Default|GetAction%20Widget) (Utilities|String|ToString(Integer) _output_get))
    (if (>= _output_get 3)
      (CallFunction|CreateFade)
      (Utilities|FlowControl|Delay 1.0)
      (Game|OpenLevel(byName) "tutorial-6"))))

(event EventShowTutorialHUD
  (params (boxType :type Integer) (text :type Set%20of%20Strings))
  (Variables|Default|SetBox%20Type boxType)
  (bind _result (Utilities|Set|ToArray text))
  (bind _output_get (Variables|Default|SetText%20Array _result))
  (Variables|Default|SetMaxIndex (Utilities|Array|Length _output_get))
  (bind _returnvalue (UserInterface|CreateWidget "/Game/Blueprints/UI/Tutorial/TutorialPrompts.TutorialPrompts_C"))
  (bind _output_get_2 (Variables|Default|SetTutorial%20Prompt _returnvalue))
  (UserInterface|Viewport|AddtoViewport _output_get_2 0)
  (Variables|Default|SetDialogueIndex 0)
  (Input|DisableInput (Game|GetPlayerCharacter 0) (Game|GetPlayerController 0))
  (if (> (Variables|Default|GetMaxIndex) 0)
    (Default|ChangeText (Variables|Default|GetTutorial%20Prompt) (Utilities|Array|Get(acopy) (Variables|Default|GetText%20Array)))
    (Default|ChangeInputText (Variables|Default|GetTutorial%20Prompt) (Variables|Default|GetInput%20Title) (Variables|Default|GetInput%20Text))))

(event EventUpdateWalls
  (bind _returnvalue (Game|GetCurrentLevelName true))
  (if (Utilities|Enum|Equal(Enum) _returnvalue "tutorial-6")
    (bind _output_get (Variables|Default|SetWalls (+ 1 (Variables|Default|GetWalls))))
    (Default|ChangeCount1 (Variables|Default|GetAction%20Widget) (Utilities|String|ToString(Integer) _output_get))
    (if (>= _output_get 4)
      (CallFunction|CreateFade)
      (Utilities|FlowControl|Delay 1.0)
      (Game|OpenLevel(byName) "tutorial-7"))))

(event EventBeginPlay
  (bind _ascapstone_game_instance (Utilities|Casting|CastToCapstoneGameInstance (Game|GetGameInstance)))
  (Utilities|IsValid _ascapstone_game_instance
    (:Is%20Valid
      (Variables|Default|SetGame%20Mode (Class|CapstoneGameInstance|GetGameMode _ascapstone_game_instance))
      (Variables|Default|SetInput%20Title "")
      (Variables|Default|SetInput%20Text ""))))

(event EventUpdateLightAttacks
  (bind _returnvalue (Game|GetCurrentLevelName true))
  (if (Utilities|Enum|Equal(Enum) _returnvalue "tutorial-1")
    (bind _output_get (Variables|Default|SetLight%20Attacks (+ 1 (Variables|Default|GetLight%20Attacks))))
    (Default|ChangeCount1 (Variables|Default|GetAction%20Widget) (Utilities|String|ToString(Integer) _output_get))
    (if (Math|Boolean|ANDBoolean (>= _output_get 2) (>= (stale EventUpdateHeavyAttacks _output_get) 2) (>= (stale EventUpdateSpecialAttacks _output_get) 1))
      (bind _newparam1 (CallFunction|CreateDialogues))
      (CallFunction|EventStartTutorialHUD _newparam1 2))))

(event EventUpdateCounterAttacks
  (bind _returnvalue (Game|GetCurrentLevelName true))
  (if (Utilities|Enum|Equal(Enum) _returnvalue "tutorial-9")
    (bind _output_get (Variables|Default|SetCounter%20Attacks (+ 1 (Variables|Default|GetCounter%20Attacks))))
    (Default|ChangeCount1 (Variables|Default|GetAction%20Widget) (Utilities|String|ToString(Integer) _output_get))
    (if (>= _output_get 3)
      (bind _newparam1 (CallFunction|CreateDialogues 4))
      (CallFunction|EventStartTutorialHUD _newparam1 7))))

(event Input|ActionEvents|InputActionProgressDialogue
  (params (Key :type Key%20Structure))
  (bind _returnvalue (Game|GetPlayerCharacter 0))
  (:Pressed
    (Utilities|IsValid (Variables|Default|GetTutorial%20Prompt)
      (:Is%20Valid
        (bind _output_get (Variables|Default|SetDialogueIndex (+ (Variables|Default|GetDialogueIndex) 1)))
        (if (< _output_get (Variables|Default|GetMaxIndex))
          (Default|ChangeText (Variables|Default|GetTutorial%20Prompt) (Utilities|Array|Get(acopy) (Variables|Default|GetText%20Array) (Variables|Default|GetDialogueIndex)))
          (elif (== (Variables|Default|GetDialogueIndex) (Variables|Default|GetMaxIndex))
            (switch int (Variables|Default|GetBox%20Type)
              (:0
                (Widget|RemovefromParent (Variables|Default|GetTutorial%20Prompt))
                (Input|EnableInput (Game|GetPlayerCharacter 0) (Game|GetPlayerController 0))
                (bind _returnvalue_2 (Game|GetCurrentLevelName true))
                (if (Utilities|Enum|NotEqual(Enum) _returnvalue_2 "tutorial-0")
                  (bind _returnvalue_3 (UserInterface|CreateWidget "/Game/Blueprints/UI/Tutorial/Tutorial_Action_1.Tutorial_Action_1_C"))
                  (bind _output_get_2 (Variables|Default|SetAction%20Widget _returnvalue_3))
                  (UserInterface|Viewport|AddtoViewport _output_get_2 0)
                  (bind _returnvalue_4 (Game|GetCurrentLevelName true))
                  (switch string _returnvalue_4
                    (:Default
                      (Default|ChangeText (Variables|Default|GetAction%20Widget) "Wall Blocks:" "" "" "0" :!label _label)
                      (Utilities|IsValid _returnvalue :!label _label_2
                        (:Is%20Valid
                          (bind _outactors (Actor|GetAllActorsOfClass "/Script/CE301CapstoneProject.EnemyBase"))
                          (for _array_element _outactors
                            (Class|FighterBase|SetTarget _array_element _returnvalue)
                            (Class|EnemyBase|GetNewTarget _array_element true)))))
                    (:tutorial-1
                      (Default|ChangeText (Variables|Default|GetAction%20Widget) "Light Attacks:" "Heavy Attacks:" "Special Attacks:" "0" "0" "0"))
                    (:tutorial-2
                      (Default|ChangeText (Variables|Default|GetAction%20Widget) "Kickboxing Attacks:" "Weapon Attacks:" "" "0" "0"))
                    (:tutorial-3
                      (Default|ChangeText (Variables|Default|GetAction%20Widget) "Magic Attacks:" "" "" "0"))
                    (:tutorial-4
                      (Default|ChangeText (Variables|Default|GetAction%20Widget) "Dodges:" "" "" "0")
                      (goto _label_2))
                    (:tutorial-5
                      (Default|ChangeText (Variables|Default|GetAction%20Widget) "Blocks:" "" "" "0")
                      (goto _label_2))
                    (:tutorial-6
                      (goto _label))
                    (:tutorial-7
                      (Default|ChangeText (Variables|Default|GetAction%20Widget) "Perfect Blocks:" "" "" "0")
                      (goto _label_2))
                    (:tutorial-8
                      (Default|ChangeText (Variables|Default|GetAction%20Widget) "Block Breakers:" "" "" "0"))
                    (:tutorial-9
                      (Default|ChangeText (Variables|Default|GetAction%20Widget) "Counter Attacks:" "" "" "0")
                      (goto _label_2)))))
              (:1
                (CallFunction|CreateFade)
                (Utilities|FlowControl|Delay 1.0)
                (Game|OpenLevel(byName) "tutorial-1"))
              (:2
                (CallFunction|CreateFade)
                (Utilities|FlowControl|Delay 1.0)
                (Game|OpenLevel(byName) "tutorial-2"))
              (:7
                (CallFunction|CreateFade)
                (Utilities|FlowControl|Delay 1.0)
                (Game|OpenLevel(byName) "MainMenu")))))))))

(fn ConstructionScript)

(fn CreateDialogues
  (params (NewParam :type Integer))
  (switch int NewParam
    (:0
      (return (LocalVariables|GetText%201)))
    (:4
      (return (LocalVariables|GetText%204)))))

(fn CreateFade
  (bind _returnvalue (UserInterface|CreateWidget "/Game/Blueprints/UI/FadeBlack.FadeBlack_C"))
  (UserInterface|Viewport|AddtoViewport _returnvalue 0)
  (Default|Fadein _returnvalue))

(fn HideActor
  (params (Actor :type Actor%20Object%20Reference))
  (Rendering|SetActorHiddenInGame Actor true))