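; BP_TutorialBox is a trigger actor that shows a tutorial widget while the player stands inside it.
; The widget component starts hidden on BeginPlay.
; Actor overlap events cast to BP_PlayerCharacter, showing the widget when the player enters and hiding it when the player leaves.
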(event EventBeginPlay
  (Rendering|SetVisibility (Variables|Default|GetWidget) false false))

(event Collision|EventActorBeginOverlap
  (params (OtherActor :type Actor%20Object%20Reference))
  (bind _asbp_player_character (Utilities|Casting|CastToBP_PlayerCharacter OtherActor))
  (Utilities|IsValid _asbp_player_character
    (:Is%20Valid
      (Rendering|SetVisibility (Variables|Default|GetWidget) true false))))

(event Collision|EventActorEndOverlap
  (params (OtherActor :type Actor%20Object%20Reference))
  (bind _asbp_player_character (Utilities|Casting|CastToBP_PlayerCharacter OtherActor))
  (Utilities|IsValid _asbp_player_character
    (:Is%20Valid
      (Rendering|SetVisibility (Variables|Default|GetWidget) false false))))

(fn ConstructionScript)